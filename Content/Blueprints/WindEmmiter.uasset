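; WindEmmiter is a wind emitter actor with a box volume extending forward from its origin, apparently an unfinished prototype.
; The construction script sizes WindVolume from WindVolumeBounds and offsets it by the X extent, so the box starts at the actor.
; Every tick it line traces on Visibility from itself to each overlapping actor, but the results are unused and no wind force is applied.
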(event EventBeginPlay)

(event Collision|EventActorBeginOverlap
  (params (OtherActor :type Actor%20Object%20Reference)))

(event EventTick
  (params (DeltaSeconds :type Float%20%28single-precision%29))
  (for _array_element (Collision|GetOverlappingActors (Variables|Default|GetWindVolume) 0 :!class /Script/Engine.PrimitiveComponent)
    (Collision|LineTraceByChannel (Transformation|GetActorLocation) (Transformation|GetActorLocation _array_element) "TraceTypeQuery1" false 0 "None")))

(fn ConstructionScript
  (bind _windvolume (Variables|Default|GetWindVolume))
  (bind _windvolumebounds (Variables|WindSettings|GetwindVolumeBounds))
  (Components|Box|SetBoxExtent _windvolume _windvolumebounds true)
  (Transformation|SetRelativeLocation _windvolume (Math|Vector|MakeVector (.X (Math|Vector|BreakVector _windvolumebounds)) 0.0 0.0) false false))